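; BP_Anim_SlashDMG is an animation notify state that deals sword slash damage during its window.
; Each tick it sphere-traces on the Camera channel between the sword's top and bottom FX sockets, with debug drawing on.
; Any hit actor not yet in DamagedEnemy is recorded and receives fixed BP_SlashParryDamage.
; The list clears when the notify begins, so each actor is damaged once per window.
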(fn `Received_NotifyBegin`
  (params (MeshComp :type "SkeletalMeshComponent Object Reference") (Animation :type "AnimSequenceBase Object Reference") (TotalDuration :type "Float (double-precision)"))
  (returns (ReturnValue :type Boolean))
  (`KismetArrayLibrary.Array_Clear` (`self.Damaged Enemy`))
  (return false))

(fn `Received_NotifyTick`
  (params (MeshComp :type "SkeletalMeshComponent Object Reference") (Animation :type "AnimSequenceBase Object Reference") (FrameDeltaTime :type "Float (double-precision)"))
  (returns (ReturnValue :type Boolean))
  (bind _outhit (`KismetSystemLibrary.SphereTraceSingle` :`WorldContextObject` MeshComp :`Start` (`SceneComponent.GetSocketLocation` MeshComp "FX_Sword_Top") :`End` (`SceneComponent.GetSocketLocation` MeshComp "FX_Sword_Bottom") :`Radius` 50.0 :`TraceChannel` "TraceTypeQuery2" :`DrawDebugType` "ForDuration" :`DrawTime` 0.3))
  (if (not (`KismetArrayLibrary.Array_Contains` (`self.Damaged Enemy`) (`.HitActor` (`GameplayStatics.BreakHitResult` _outhit))))
    (`KismetArrayLibrary.Array_Add` (`self.Damaged Enemy`) (`.HitActor` (`GameplayStatics.BreakHitResult` _outhit)))
    (`GameplayStatics.ApplyDamage` (`.HitActor` (`GameplayStatics.BreakHitResult` _outhit)) 33.400002 null null "/Game/Blueprints/BP_SlashParryDamage.BP_SlashParryDamage_C")
    (`KismetSystemLibrary.PrintString` null "Dealt Damage")
    (return false)
    (else
      (return false))))