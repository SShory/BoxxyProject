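; BP_EnemyShot is an enemy projectile that damages the player and can be parried back at enemies.
; On hitbox overlap with a SideScrollerCharacter, a "parry" tag on its ParryBox triggers a deflect; otherwise the shot damages a "player"-tagged actor.
; Deflecting swaps the material, reverses velocity and enables higher damage against "enemy"-tagged actors.
; It is destroyed on a damaging hit or after a short lifetime.
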(event `self.ReceiveBeginPlay`
  (`KismetSystemLibrary.Delay` 5.0)
  (`self.K2_DestroyActor`))

(event `self.Hitbox.OnComponentBeginOverlap`
  (params (OverlappedComponent :type "PrimitiveComponent Object Reference") (OtherActor :type "Actor Object Reference") (OtherComp :type "PrimitiveComponent Object Reference") (OtherBodyIndex :type Integer) (bFromSweep :type Boolean) (SweepResult :type "HitResult Structure (by ref)"))
  (`|ExecutionSequence`
    (:`then_0`
      (bind _asside_scroller_character (cast `/Game/SideScrollerBP/Blueprints/SideScrollerCharacter` OtherActor))
      (if (`ActorComponent.ComponentHasTag` (`/Game/SideScrollerBP/Blueprints/SideScrollerCharacter.parryBox` _asside_scroller_character) "parry")
        (`self.deflect`)
        (elif (`self.ActorHasTag` OtherActor "player")
          (`GameplayStatics.ApplyDamage` OtherActor 10.0)
          (`self.K2_DestroyActor`))))
    (:`then_1`
      (if (`self.isDeflected`)
        (if (`self.ActorHasTag` OtherActor "enemy")
          (`GameplayStatics.ApplyDamage` OtherActor 25.0)
          (set `self.isDeflected` false)
          (`self.K2_DestroyActor`))))))

(event `self.ReceiveAnyDamage`
  (params (Damage :type "Float (single-precision)") (DamageType :type "DamageType Object Reference") (InstigatedBy :type "Controller Object Reference") (DamageCauser :type "Actor Object Reference"))
  (`KismetSystemLibrary.PrintString` "ching"))

(event `deflect`
  (bind _projectilemovement (`self.ProjectileMovement`))
  (`PrimitiveComponent.SetMaterial` (`self.Projectile`) 0 "/Game/Materials/M_BlasterProjectile.M_BlasterProjectile")
  (set `MovementComponent.Velocity` (* (`MovementComponent.Velocity` _projectilemovement) -1) _projectilemovement)
  (set `self.isDeflected` true))

(fn `UserConstructionScript`)